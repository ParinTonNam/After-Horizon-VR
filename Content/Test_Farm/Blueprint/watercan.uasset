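; Watering can actor for a farm game that spends water when its box overlaps a planted crop.
; If its blue flag is set and the main game mode has water left, overlap turns the mesh blue and decrements the shared water limit.
; A cooldown flag blocks repeat use until any end overlap clears it and restores the chrome material.
; The crop itself is not modified here.
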(event `self.ReceiveTick`
  (params (DeltaSeconds :type "Float (single-precision)")))

(event `self.Box.OnComponentBeginOverlap`
  (params (OverlappedComponent :type "PrimitiveComponent Object Reference") (OtherActor :type "Actor Object Reference") (OtherComp :type "PrimitiveComponent Object Reference") (OtherBodyIndex :type Integer) (bFromSweep :type Boolean) (SweepResult :type "HitResult Structure (by ref)"))
  (set `self.overlap` true)
  (bind _asmain (cast `/Game/Test_Farm/Blueprint/main` (`GameplayStatics.GetGameMode`)))
  (bind _water_limit (`/Game/Test_Farm/Blueprint/main.water limit` _asmain))
  (if (and (`self.isblue`) (> _water_limit 0))
    (if (not (`self.coodown`))
      (bind _ascrop (cast `/Game/Test_Farm/Blueprint/crop` OtherActor))
      (if (`/Game/Test_Farm/Blueprint/crop.isPlant` _ascrop)
        (`PrimitiveComponent.SetMaterial` (`self.StaticMesh`) 0 "/Game/LevelPrototyping/Materials/MI_Solid_Blue.MI_Solid_Blue")
        (set `/Game/Test_Farm/Blueprint/main.water limit` (- _water_limit 1) _asmain)
        (set `self.coodown` true)))))

(event `self.Box.OnComponentEndOverlap`
  (params (OverlappedComponent :type "PrimitiveComponent Object Reference") (OtherActor :type "Actor Object Reference") (OtherComp :type "PrimitiveComponent Object Reference") (OtherBodyIndex :type Integer))
  (set `self.overlap` false)
  (`PrimitiveComponent.SetMaterial` (`self.StaticMesh`) 0 "/Game/StarterContent/Materials/M_Metal_Chrome.M_Metal_Chrome")
  (set `self.coodown` false))

(fn `UserConstructionScript`)