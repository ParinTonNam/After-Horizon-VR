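; Pipe tile actor for a water-flow rotation puzzle, with Type selecting mesh, open sides and the yellow goal variant.
; Openings are North/East/South/West booleans, which ChangeDirection updates per type to represent a turn.
; Every Tick re-derives WaterFill from StartWater or a filled NearPipe neighbour with a matching opening, so flow propagates by polling.
; Red pipes get a red overlay and cannot rotate; a shake event jiggles the box.
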(event `self.ReceiveBeginPlay`
  (bind _staticmesh (`self.StaticMesh`))
  ;[1 1 1] Set Pipe Type
  (switch `int` (`self.type`)
    (:`Default`
      (`self.set pipe` "/Game/Test_Farm/Blueprint/pipe/materials/green_t.green_t" "/Game/Test_Farm/pipe/titreiwhx_LOD1.titreiwhx_LOD1" false true true :!label _label)
      (`SceneComponent.K2_SetRelativeLocation` (`self.StaticMesh`) (-30.0 0.0 0.0) false false))
    (:`1`
      (`self.set pipe` "/Game/Test_Farm/Blueprint/pipe/materials/green_t.green_t" "/Game/Test_Farm/pipe/tiwidimhx_LOD2.tiwidimhx_LOD2" true false true)
      (`SceneComponent.SetRelativeScale3D` (`self.StaticMesh`) (0.5 1.5 1.5))
      (`SceneComponent.K2_SetRelativeLocation` (`self.StaticMesh`) (-25.0 0.0 0.0) false false))
    (:`2`
      (goto _label))
    (:`3`
      (`self.set pipe` "/Game/Test_Farm/Blueprint/pipe/materials/green_t.green_t" "/Game/Test_Farm/pipe/titsbhrhx_LOD5.titsbhrhx_LOD5" true)
      (`SceneComponent.K2_SetRelativeLocation` (`self.StaticMesh`) (-32.0 0.0 0.0) false false))
    (:`4`
      (`self.set pipe` "/Game/Test_Farm/Blueprint/pipe/materials/green_t.green_t" "/Game/Test_Farm/pipe/tjejbfyhx_LOD6.tjejbfyhx_LOD6")
      (`SceneComponent.K2_SetRelativeLocation` (`self.StaticMesh`) (-32.0 0.0 0.0) false false))
    (:`5`
      (`self.set pipe` "/Game/Test_Farm/Blueprint/pipe/materials/yellow_t.yellow_t" "/Game/Test_Farm/pipe/tiwicjehx_LOD0.tiwicjehx_LOD0" true true true true)
      (`SceneComponent.SetRelativeScale3D` _staticmesh (1.5 1.5 2.0))
      (`SceneComponent.K2_SetRelativeRotation` _staticmesh (struct :`Yaw` 90.0 :`Roll` -90.0) false false)
      (`SceneComponent.K2_SetRelativeLocation` _staticmesh (-25.0 0.0 0.0) false false)
      (set `self.goal_pipe` true)
      (set `self.north` true)
      (set `self.east` true)
      (set `self.south` true)
      (set `self.west` true))))

(event `self.ReceiveTick`
  (params (DeltaSeconds :type "Float (single-precision)"))
  ;[1 1 1] Check Pipe Status
  (if (`self.start_water`)
    (set `self.water_fill` true)
    (else
      (set `self.water_fill` false)))
  (`self.process_pipe`)
  (`MeshComponent.SetOverlayMaterial` (`self.StaticMesh`) null)
  (`MeshComponent.SetOverlayMaterial` (`self.right`) null)
  (`MeshComponent.SetOverlayMaterial` (`self.down`) null)
  (`MeshComponent.SetOverlayMaterial` (`self.left`) null)
  (`MeshComponent.SetOverlayMaterial` (`self.up`) null)
  (if (`self.red_pipe`)
    (`MeshComponent.SetOverlayMaterial` (`self.StaticMesh`) "/Game/Test_Farm/Blueprint/pipe/materials/red_t.red_t")
    (`MeshComponent.SetOverlayMaterial` (`self.right`) "/Game/Test_Farm/Blueprint/pipe/materials/red_t.red_t")
    (`MeshComponent.SetOverlayMaterial` (`self.down`) "/Game/Test_Farm/Blueprint/pipe/materials/red_t.red_t")
    (`MeshComponent.SetOverlayMaterial` (`self.left`) "/Game/Test_Farm/Blueprint/pipe/materials/red_t.red_t")
    (`MeshComponent.SetOverlayMaterial` (`self.up`) "/Game/Test_Farm/Blueprint/pipe/materials/red_t.red_t")
    (set `self.can_rotate` false)
    (elif (not (`self.goal_pipe`))
      (set `self.can_rotate` true))))

(event `process_pipe`
  ;[1 1 1] Water Flow in Pipe
  (for (_array_element _array_index) (`self.near_pipe`)
    (`/Engine/EditorBlueprintResources/StandardMacros.IsValid` _array_element
      (:`Is Valid`
        (switch `int` _array_index
          (:`0`
            (bind _start_water (`/Game/Test_Farm/Blueprint/pipe/pipe_main.start_water` _array_element))
            (if (and (`self.north`) (or (`/Game/Test_Farm/Blueprint/pipe/pipe_main.south` _array_element) _start_water))
              (if (or (`/Game/Test_Farm/Blueprint/pipe/pipe_main.water_fill` _array_element) (`/Game/Test_Farm/Blueprint/pipe/pipe_main.start_water` _array_element)) :!label _label_2
                (set `self.water_fill` true)
                (break)
                (else
                  _))))
          (:`1`
            (if (and (`self.east`) (or (`/Game/Test_Farm/Blueprint/pipe/pipe_main.west` _array_element) _start_water))
              (goto _label_2)
              (else
                _)))
          (:`2`
            (if (and (`self.west`) (or (`/Game/Test_Farm/Blueprint/pipe/pipe_main.east` _array_element) _start_water))
              (goto _label_2)
              (else
                _)))
          (:`3`
            (if (and (`self.south`) (or (`/Game/Test_Farm/Blueprint/pipe/pipe_main.north` _array_element) _start_water))
              (goto _label_2)
              (else
                _))))
        (set `self.water_fill` false)))))

(event `shake`
  (bind _box_0 (`self.box_0`))
  (bind (_returnvalue_location _returnvalue_rotation) (`KismetMathLibrary.BreakTransform` (`SceneComponent.GetRelativeTransform` _box_0)))
  ;[1 1 1] Click Red Pipe
  (`KismetSystemLibrary.MoveComponentTo` _box_0 (+ _returnvalue_location (5.0 0.0 0.0)) _returnvalue_rotation false false 0.01)
  (`KismetSystemLibrary.Delay` 0.01)
  (`KismetSystemLibrary.MoveComponentTo` _box_0 (+ _returnvalue_location (0.0 5.0 0.0)) _returnvalue_rotation false false 0.01)
  (`KismetSystemLibrary.Delay` 0.01)
  (`KismetSystemLibrary.MoveComponentTo` _box_0 (+ _returnvalue_location (-5.0 0.0 0.0)) _returnvalue_rotation false false 0.01)
  (`KismetSystemLibrary.Delay` 0.01)
  (`KismetSystemLibrary.MoveComponentTo` _box_0 (+ _returnvalue_location (0.0 -5.0 0.0)) _returnvalue_rotation false false 0.01))

(fn `change direction`
  (switch `int` (`self.type`)
    (:`1`
      ;[1 1 1] pipe type1
      (set `self.north` (not (`self.north`)))
      (set `self.east` (not (`self.east`)))
      (set `self.south` (not (`self.south`)))
      (set `self.west` (not (`self.west`))))
    (:`2`
      ;[1 1 1] pipe type 2
      (if (and (`self.north`) (`self.east`))
        (set `self.north` false)
        (set `self.south` true)
        (elif (and (`self.east`) (`self.south`))
          (set `self.east` false)
          (set `self.west` true)
          (elif (and (`self.south`) (`self.west`))
            (set `self.south` false)
            (set `self.north` true)
            (elif (and (`self.west`) (`self.north`))
              (set `self.west` false)
              (set `self.east` true))))))
    (:`3`
      ;[1 1 1] pipe type 3
      (if (not (`self.south`))
        (set `self.west` false)
        (set `self.south` true)
        (elif (not (`self.west`))
          (set `self.north` false)
          (set `self.west` true)
          (elif (not (`self.north`))
            (set `self.east` false)
            (set `self.north` true)
            (elif (not (`self.east`))
              (set `self.south` false)
              (set `self.east` true))))))))

(fn `set pipe`
  (params (Material :type "MaterialInterface Object Reference") (NewMesh :type "StaticMesh Object Reference") (down_show :type Boolean) (left_show :type Boolean) (up_show :type Boolean) (right_show :type Boolean))
  (bind _staticmesh (`self.StaticMesh`))
  ;[1 1 1] Set mesh
  (`PrimitiveComponent.SetMaterial` _staticmesh 0 Material)
  (`StaticMeshComponent.SetStaticMesh` _staticmesh NewMesh)
  (`SceneComponent.SetHiddenInGame` (`self.right`) right_show false)
  (`SceneComponent.SetHiddenInGame` (`self.down`) down_show false)
  (`SceneComponent.SetHiddenInGame` (`self.left`) left_show false)
  (`SceneComponent.SetHiddenInGame` (`self.up`) up_show false)
  ;[1 1 1] set condition for water flow
  (set `self.north` (not down_show))
  (set `self.east` (not left_show))
  (set `self.south` (not up_show))
  (set `self.west` (not right_show)))

(fn `UserConstructionScript`)