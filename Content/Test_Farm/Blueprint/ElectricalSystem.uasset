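; Bunker electrical fuse puzzle: while unfixed, it drains the game mode's BunkerHealth.
; Box overlaps place the carried fuse and check it against Order, advancing Count and five red/green progress lights, or resetting.
; A delay-throttled Tick blinks a BlinkOrder light and runs a countdown that resets progress; a physical button also resets, respawning five fuses.
; CheckIsFix marks it repaired at five correct fuses, but nothing here calls it.
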(event `broken`
  (if (`self.boom`)
    (set `self.is_fix_electric` false)
    (`self.reset`)))

(event `self.ReceiveTick`
  (params (DeltaSeconds :type "Float (single-precision)"))
  (if (not (`self.is_fix_electric`))
    (`KismetSystemLibrary.Delay` 0.5)
    (`self.blink`)
    (`KismetSystemLibrary.Delay` 1.0)
    (bind _asmain (cast `/Game/Test_Farm/Blueprint/main` (`GameplayStatics.GetGameMode`)))
    (bind _returnvalue (- (`/Game/Test_Farm/Blueprint/main.bunker_health` _asmain) 1))
    (if (<= _returnvalue 0)
      (set `/Game/Test_Farm/Blueprint/main.bunker_health` 0 _asmain)
      (else
        (set `/Game/Test_Farm/Blueprint/main.bunker_health` _returnvalue _asmain)))
    (`TextRenderComponent.K2_SetText` (`self.TextRender`) (`KismetTextLibrary.Conv_IntToText` (`/Game/Test_Farm/Blueprint/main.bunker_health` _asmain)))
    (if (> (`self.count`) 0)
      (if (<= (`self.Time_10`) 0)
        (`self.reset`)
        (bind _output_get (set `self.Time_10` 15))
        (`TextRenderComponent.K2_SetText` (`self.time`) (`KismetTextLibrary.Conv_IntToText` _output_get))
        (else
          (bind _output_get_2 (set `self.Time_10` (- (`self.Time_10`) 1)))
          (`TextRenderComponent.K2_SetText` (`self.time`) (`KismetTextLibrary.Conv_IntToText` _output_get_2)))))))

(event `self.Box1.OnComponentBeginOverlap`
  (params (OverlappedComponent :type "PrimitiveComponent Object Reference") (OtherActor :type "Actor Object Reference") (OtherComp :type "PrimitiveComponent Object Reference") (OtherBodyIndex :type Integer) (bFromSweep :type Boolean) (SweepResult :type "HitResult Structure (by ref)"))
  (`self.fill_fuse` (`self.fuse1`))
  (`self.check_order` 1))

(event `self.Box2.OnComponentBeginOverlap`
  (params (OverlappedComponent :type "PrimitiveComponent Object Reference") (OtherActor :type "Actor Object Reference") (OtherComp :type "PrimitiveComponent Object Reference") (OtherBodyIndex :type Integer) (bFromSweep :type Boolean) (SweepResult :type "HitResult Structure (by ref)"))
  (`self.fill_fuse` (`self.fuse2`))
  (`self.check_order` 2))

(event `self.Box3.OnComponentBeginOverlap`
  (params (OverlappedComponent :type "PrimitiveComponent Object Reference") (OtherActor :type "Actor Object Reference") (OtherComp :type "PrimitiveComponent Object Reference") (OtherBodyIndex :type Integer) (bFromSweep :type Boolean) (SweepResult :type "HitResult Structure (by ref)"))
  (`self.fill_fuse` (`self.fuse3`))
  (`self.check_order` 3))

(event `self.Box4.OnComponentBeginOverlap`
  (params (OverlappedComponent :type "PrimitiveComponent Object Reference") (OtherActor :type "Actor Object Reference") (OtherComp :type "PrimitiveComponent Object Reference") (OtherBodyIndex :type Integer) (bFromSweep :type Boolean) (SweepResult :type "HitResult Structure (by ref)"))
  (`self.fill_fuse` (`self.fuse4`))
  (`self.check_order` 4))

(event `self.Box5.OnComponentBeginOverlap`
  (params (OverlappedComponent :type "PrimitiveComponent Object Reference") (OtherActor :type "Actor Object Reference") (OtherComp :type "PrimitiveComponent Object Reference") (OtherBodyIndex :type Integer) (bFromSweep :type Boolean) (SweepResult :type "HitResult Structure (by ref)"))
  (`self.fill_fuse` (`self.fuse5`))
  (`self.check_order` 5))

(event `self.Box6.OnComponentBeginOverlap`
  (params (OverlappedComponent :type "PrimitiveComponent Object Reference") (OtherActor :type "Actor Object Reference") (OtherComp :type "PrimitiveComponent Object Reference") (OtherBodyIndex :type Integer) (bFromSweep :type Boolean) (SweepResult :type "HitResult Structure (by ref)"))
  (`self.fill_fuse` (`self.fuse6`))
  (`self.check_order` 6))

(event `self.Box7.OnComponentBeginOverlap`
  (params (OverlappedComponent :type "PrimitiveComponent Object Reference") (OtherActor :type "Actor Object Reference") (OtherComp :type "PrimitiveComponent Object Reference") (OtherBodyIndex :type Integer) (bFromSweep :type Boolean) (SweepResult :type "HitResult Structure (by ref)"))
  (`self.fill_fuse` (`self.fuse7`))
  (`self.check_order` 7))

(event `self.Box8.OnComponentBeginOverlap`
  (params (OverlappedComponent :type "PrimitiveComponent Object Reference") (OtherActor :type "Actor Object Reference") (OtherComp :type "PrimitiveComponent Object Reference") (OtherBodyIndex :type Integer) (bFromSweep :type Boolean) (SweepResult :type "HitResult Structure (by ref)"))
  (`self.fill_fuse` (`self.fuse8`))
  (`self.check_order` 8))

(event `self.Box9.OnComponentBeginOverlap`
  (params (OverlappedComponent :type "PrimitiveComponent Object Reference") (OtherActor :type "Actor Object Reference") (OtherComp :type "PrimitiveComponent Object Reference") (OtherBodyIndex :type Integer) (bFromSweep :type Boolean) (SweepResult :type "HitResult Structure (by ref)"))
  (`self.fill_fuse` (`self.fuse9`))
  (`self.check_order` 9))

(event `self.Box10.OnComponentBeginOverlap`
  (params (OverlappedComponent :type "PrimitiveComponent Object Reference") (OtherActor :type "Actor Object Reference") (OtherComp :type "PrimitiveComponent Object Reference") (OtherBodyIndex :type Integer) (bFromSweep :type Boolean) (SweepResult :type "HitResult Structure (by ref)"))
  (`self.fill_fuse` (`self.fuse10`))
  (`self.check_order` 10))

(event `self.Btn _coliision.OnComponentBeginOverlap`
  (params (OverlappedComponent :type "PrimitiveComponent Object Reference") (OtherActor :type "Actor Object Reference") (OtherComp :type "PrimitiveComponent Object Reference") (OtherBodyIndex :type Integer) (bFromSweep :type Boolean) (SweepResult :type "HitResult Structure (by ref)"))
  (bind _reset_btn (`self.reset_btn`))
  (bind _reset_btn_2 (`self.reset_btn`))
  (if (not (`self.is_press`))
    (set `self.is_press` true)
    (`KismetSystemLibrary.MoveComponentTo` _reset_btn_2 (+ (`SceneComponent.RelativeLocation` _reset_btn_2) (0.0 -0.4 0.0)))
    (`self.reset`)
    (`KismetSystemLibrary.MoveComponentTo` _reset_btn (+ (`SceneComponent.RelativeLocation` _reset_btn) (0.0 0.4 0.0)))
    (`self.turn_on_light`)
    (set `self.is_press` false)))

(fn `blink`
  (bind _blink10 (`self.blink10`))
  (if (>= (`self.count`) 1)
    (if (`self.on_off`)
      (`LightComponent.SetIntensity` (`|GetArrayItem` (`|MakeArray` (`self.blink1`) (`self.blink2`) (`self.blink3`) (`self.blink4`) (`self.blink5`) (`self.blink6`) (`self.blink7`) (`self.blink8`) (`self.blink9`) _blink10) (- (`|GetArrayItem` (`self.blink_order`) (- (`self.count`) 1)) 1)) 500.0)
      (set `self.on_off` false)
      (else
        (`LightComponent.SetIntensity` _blink10 0.0 :!label _label)
        (`LightComponent.SetIntensity` (`self.blink9`) 0.0)
        (`LightComponent.SetIntensity` (`self.blink8`) 0.0)
        (`LightComponent.SetIntensity` (`self.blink7`) 0.0)
        (`LightComponent.SetIntensity` (`self.blink6`) 0.0)
        (`LightComponent.SetIntensity` (`self.blink5`) 0.0)
        (`LightComponent.SetIntensity` (`self.blink4`) 0.0)
        (`LightComponent.SetIntensity` (`self.blink3`) 0.0)
        (`LightComponent.SetIntensity` (`self.blink2`) 0.0)
        (`LightComponent.SetIntensity` (`self.blink1`) 0.0)
        (set `self.on_off` true)))
    (else
      (goto _label))))

(fn `Check Is Fix`
  (if (`self.boom`)
    (if (>= (`self.count`) 5)
      (set `self.boom` false)
      (set `self.is_fix_electric` true)
      (else
        (set `self.boom` true)
        (set `self.is_fix_electric` false)))))

(fn `check_order`
  (params (number :type Integer))
  (bind _asmain (cast `/Game/Test_Farm/Blueprint/main` (`GameplayStatics.GetGameMode`)))
  (if (`/Game/Test_Farm/Blueprint/main.is_grab_fuse` _asmain)
    (if (== number (`|GetArrayItem` (`self.order`) (`self.count`)))
      (set `self.count` (+ (`self.count`) 1))
      (else
        (`self.reset`)))
    (set `/Game/Test_Farm/Blueprint/main.is_grab_fuse` false _asmain)
    (`self.turn_on_light`)
    (set `self.Time_10` 15)))

(fn `fill_fuse`
  (params (Target :type "SceneComponent Object Reference"))
  (bind _asmain (cast `/Game/Test_Farm/Blueprint/main` (`GameplayStatics.GetGameMode`)))
  (if (`/Game/Test_Farm/Blueprint/main.is_grab_fuse` _asmain)
    (`SceneComponent.SetHiddenInGame` Target false false)
    (`self.K2_DestroyActor` (`/Game/Test_Farm/Blueprint/main.Fuse` _asmain))))

(fn `reset`
  (`SceneComponent.SetHiddenInGame` (`self.fuse1`) true false)
  (`SceneComponent.SetHiddenInGame` (`self.fuse2`) true false)
  (`SceneComponent.SetHiddenInGame` (`self.fuse3`) true false)
  (`SceneComponent.SetHiddenInGame` (`self.fuse4`) true false)
  (`SceneComponent.SetHiddenInGame` (`self.fuse5`) true false)
  (`SceneComponent.SetHiddenInGame` (`self.fuse6`) true false)
  (`SceneComponent.SetHiddenInGame` (`self.fuse7`) true false)
  (`SceneComponent.SetHiddenInGame` (`self.fuse8`) true false)
  (`SceneComponent.SetHiddenInGame` (`self.fuse9`) true false)
  (`SceneComponent.SetHiddenInGame` (`self.fuse10`) true false)
  (bind _outactors (`GameplayStatics.GetAllActorsOfClass` "/Game/Test_Farm/Blueprint/fuse.fuse_C"))
  (for _array_element _outactors
    (`self.K2_DestroyActor` _array_element))
  (for _index (range 5)
    (`|SpawnActorFromClass` "/Game/Test_Farm/Blueprint/fuse.fuse_C" (`KismetMathLibrary.MakeTransform` (`KismetMathLibrary.MakeVector` (`KismetMathLibrary.Conv_IntToDouble` (+ (* _index 20) 210)) -450.0 70.0) (struct :`Pitch` 90.0 :`Yaw` 180.0 :`Roll` 90.0)) "Undefined" "MultiplyWithRoot" null null))
  (set `self.count` 0)
  (set `self.Time_10` 15))

(fn `turn_on_light`
  (switch `int` (`self.count`)
    (:`0`
      (`LightComponent.SetLightColor` (`self.PointLight1`) (struct :`R` 1.0 :`A` 1.0) true)
      (`LightComponent.SetLightColor` (`self.PointLight2`) (struct :`R` 1.0 :`A` 1.0) true)
      (`LightComponent.SetLightColor` (`self.PointLight3`) (struct :`R` 1.0 :`A` 1.0) true)
      (`LightComponent.SetLightColor` (`self.PointLight4`) (struct :`R` 1.0 :`A` 1.0) true)
      (`LightComponent.SetLightColor` (`self.PointLight5`) (struct :`R` 1.0 :`A` 1.0) true))
    (:`1`
      (`LightComponent.SetLightColor` (`self.PointLight1`) (struct :`G` 1.0 :`A` 1.0) true))
    (:`2`
      (`LightComponent.SetLightColor` (`self.PointLight2`) (struct :`G` 1.0 :`A` 1.0) true)
      (`LightComponent.SetLightColor` (`self.PointLight1`) (struct :`G` 1.0 :`A` 1.0) true))
    (:`3`
      (`LightComponent.SetLightColor` (`self.PointLight1`) (struct :`G` 1.0 :`A` 1.0) true)
      (`LightComponent.SetLightColor` (`self.PointLight2`) (struct :`G` 1.0 :`A` 1.0) true)
      (`LightComponent.SetLightColor` (`self.PointLight3`) (struct :`G` 1.0 :`A` 1.0) true))
    (:`4`
      (`LightComponent.SetLightColor` (`self.PointLight1`) (struct :`G` 1.0 :`A` 1.0) true)
      (`LightComponent.SetLightColor` (`self.PointLight2`) (struct :`G` 1.0 :`A` 1.0) true)
      (`LightComponent.SetLightColor` (`self.PointLight3`) (struct :`G` 1.0 :`A` 1.0) true)
      (`LightComponent.SetLightColor` (`self.PointLight4`) (struct :`G` 1.0 :`A` 1.0) true))
    (:`5`
      (`LightComponent.SetLightColor` (`self.PointLight1`) (struct :`G` 1.0 :`A` 1.0) true)
      (`LightComponent.SetLightColor` (`self.PointLight2`) (struct :`G` 1.0 :`A` 1.0) true)
      (`LightComponent.SetLightColor` (`self.PointLight3`) (struct :`G` 1.0 :`A` 1.0) true)
      (`LightComponent.SetLightColor` (`self.PointLight4`) (struct :`G` 1.0 :`A` 1.0) true)
      (`LightComponent.SetLightColor` (`self.PointLight5`) (struct :`G` 1.0 :`A` 1.0) true))))

(fn `UserConstructionScript`)