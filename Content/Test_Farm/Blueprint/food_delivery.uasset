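; Food delivery Blueprint that converts plant actors entering its box trigger into health on the main game mode.
; On overlap, it casts the actor to plant and adjusts HarvestHealth and BunkerHealth, then destroys the plant.
; Plant number 1 adds a larger bonus to both values.
; Other plants add a smaller bonus to HarvestHealth, but set BunkerHealth from the updated HarvestHealth rather than its own value.
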(event `self.Box.OnComponentBeginOverlap`
  (params (OverlappedComponent :type "PrimitiveComponent Object Reference") (OtherActor :type "Actor Object Reference") (OtherComp :type "PrimitiveComponent Object Reference") (OtherBodyIndex :type Integer) (bFromSweep :type Boolean) (SweepResult :type "HitResult Structure (by ref)"))
  (bind _asplant (cast `/Game/Test_Farm/Blueprint/plant` OtherActor))
  (bind _asmain (cast `/Game/Test_Farm/Blueprint/main` (`GameplayStatics.GetGameMode`)))
  (if (== (`/Game/Test_Farm/Blueprint/plant.plant number` _asplant) 1)
    (set `/Game/Test_Farm/Blueprint/main.harvest_health` (+ (`/Game/Test_Farm/Blueprint/main.harvest_health` _asmain) 6) _asmain)
    (set `/Game/Test_Farm/Blueprint/main.bunker_health` (+ 6 (`/Game/Test_Farm/Blueprint/main.bunker_health` _asmain)) _asmain)
    (`self.K2_DestroyActor` OtherActor)
    (else
      (bind _output_get (set `/Game/Test_Farm/Blueprint/main.harvest_health` (+ (`/Game/Test_Farm/Blueprint/main.harvest_health` _asmain) 2) _asmain))
      (set `/Game/Test_Farm/Blueprint/main.bunker_health` (+ _output_get 2) _asmain)
      (`self.K2_DestroyActor` OtherActor))))

(fn `UserConstructionScript`)