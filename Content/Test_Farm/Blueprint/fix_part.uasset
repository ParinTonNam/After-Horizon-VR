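; Actor Blueprint for a numbered part, shown as one of four static meshes or as an empty mesh.
; Every Tick it switches on PartNumber and reapplies the matching mesh to its StaticMesh component, with zero clearing it.
; A custom spawn event uses MoveComponentTo to raise the mesh slightly along Z from its current relative location.
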(event `self.ReceiveTick`
  (params (DeltaSeconds :type "Float (single-precision)"))
  (switch `int` (`self.part_number`)
    (:`0`
      (`StaticMeshComponent.SetStaticMesh` (`self.StaticMesh`) null))
    (:`1`
      (`StaticMeshComponent.SetStaticMesh` (`self.StaticMesh`) "/Game/Test_Farm/Blueprint/part/part1/part-1-hp__3_.part-1-hp__3_"))
    (:`2`
      (`StaticMeshComponent.SetStaticMesh` (`self.StaticMesh`) "/Game/Test_Farm/Blueprint/part/part2/part-2-hp__2_.part-2-hp__2_"))
    (:`3`
      (`StaticMeshComponent.SetStaticMesh` (`self.StaticMesh`) "/Game/Test_Farm/Blueprint/part/part3/part-3-hp__1_.part-3-hp__1_"))
    (:`4`
      (`StaticMeshComponent.SetStaticMesh` (`self.StaticMesh`) "/Game/Test_Farm/Blueprint/mesh/part-4-hp.part-4-hp"))))

(event `spawn`
  (bind _staticmesh (`self.StaticMesh`))
  (`KismetSystemLibrary.MoveComponentTo` _staticmesh (+ (`SceneComponent.RelativeLocation` _staticmesh) (0.0 0.0 20.0))))

(fn `UserConstructionScript`)