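; Trigger volume at a bunker entry on the test farm that reveals the Bunker_spawn actor while the VR pawn is inside.
; When a VRPawnNew begins overlapping the Collision component, it unhides the first Bunker_spawn found in the level and turns on the pawn's right-hand widget interaction debug display.
; Ending the overlap hides the actor and turns the debug display off again.
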(event `self.collision.OnComponentBeginOverlap`
  (params (OverlappedComponent :type "PrimitiveComponent Object Reference") (OtherActor :type "Actor Object Reference") (OtherComp :type "PrimitiveComponent Object Reference") (OtherBodyIndex :type Integer) (bFromSweep :type Boolean) (SweepResult :type "HitResult Structure (by ref)"))
  (bind _asvrpawn_new (cast `/Game/Test_Farm/Blueprint/VRPawnNew` OtherActor))
  (bind _returnvalue (`GameplayStatics.GetActorOfClass` "/Game/Test_Farm/Blueprint/widget/bunker_spawn.bunker_spawn_C"))
  (`self.SetActorHiddenInGame` _returnvalue false)
  (set `WidgetInteractionComponent.bShowDebug` true (`/Game/Test_Farm/Blueprint/VRPawnNew.WidgetInteractionRight` _asvrpawn_new)))

(event `self.collision.OnComponentEndOverlap`
  (params (OverlappedComponent :type "PrimitiveComponent Object Reference") (OtherActor :type "Actor Object Reference") (OtherComp :type "PrimitiveComponent Object Reference") (OtherBodyIndex :type Integer))
  (bind _asvrpawn_new (cast `/Game/Test_Farm/Blueprint/VRPawnNew` OtherActor))
  (bind _returnvalue (`GameplayStatics.GetActorOfClass` "/Game/Test_Farm/Blueprint/widget/bunker_spawn.bunker_spawn_C"))
  (`self.SetActorHiddenInGame` _returnvalue true)
  (set `WidgetInteractionComponent.bShowDebug` false (`/Game/Test_Farm/Blueprint/VRPawnNew.WidgetInteractionRight` _asvrpawn_new)))

(fn `UserConstructionScript`)