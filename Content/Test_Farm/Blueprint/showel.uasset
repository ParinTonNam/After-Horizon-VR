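; A grabbable shovel for the farm test that registers digs on diggable actors tracked by the `main` game mode.
; While DigLimit remains, a Box overlap matching a Digable entry by display name removes that entry and turns the shovel yellow.
; The next end overlap from any actor decrements DigLimit and restores the material.
; Grab events set IsShowel, but digging never checks it.
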(event `self.GrabComponent.OnGrabbed`
  (set `self.is_showel` true))

(event `self.GrabComponent.OnDropped`
  (set `self.is_showel` false))

(event `self.Box.OnComponentBeginOverlap`
  (params (OverlappedComponent :type "PrimitiveComponent Object Reference") (OtherActor :type "Actor Object Reference") (OtherComp :type "PrimitiveComponent Object Reference") (OtherBodyIndex :type Integer) (bFromSweep :type Boolean) (SweepResult :type "HitResult Structure (by ref)"))
  (bind _asmain (cast `/Game/Test_Farm/Blueprint/main` (`GameplayStatics.GetGameMode`)))
  (bind _digable (`/Game/Test_Farm/Blueprint/main.digable` _asmain))
  (for (_array_element _array_index) _digable
    (if (`KismetStringLibrary.EqualEqual_StrStr` (`KismetSystemLibrary.GetDisplayName` OtherActor) (`KismetSystemLibrary.GetDisplayName` _array_element))
      (if (> (`/Game/Test_Farm/Blueprint/main.dig_limit` _asmain) 0)
        (if (not (`self.overlab`))
          (set `self.overlab` true)
          (`PrimitiveComponent.SetMaterial` (`self.StaticMesh`) 0 "/Game/Test_Farm/Blueprint/pipe/materials/yellow.yellow")
          (`KismetArrayLibrary.Array_Remove` _digable _array_index)
          (break))))))

(event `self.Box.OnComponentEndOverlap`
  (params (OverlappedComponent :type "PrimitiveComponent Object Reference") (OtherActor :type "Actor Object Reference") (OtherComp :type "PrimitiveComponent Object Reference") (OtherBodyIndex :type Integer))
  (if (`self.overlab`)
    (set `self.overlab` false)
    (bind _asmain (cast `/Game/Test_Farm/Blueprint/main` (`GameplayStatics.GetGameMode`)))
    (set `/Game/Test_Farm/Blueprint/main.dig_limit` (- (`/Game/Test_Farm/Blueprint/main.dig_limit` _asmain) 1) _asmain)
    (`PrimitiveComponent.SetMaterial` (`self.StaticMesh`) 0 "/Game/Farming_And_Mining/Materials/Shovel_Old_MI.Shovel_Old_MI")
    (if (>= (`self.can dig`) 1)
      (set `self.can dig` 0))))

(fn `UserConstructionScript`)