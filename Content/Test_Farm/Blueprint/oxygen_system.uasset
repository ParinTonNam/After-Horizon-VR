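; Oxygen system actor for the bunker that can break and be repaired with fix parts.
; The brok event marks it broken and halves BunkerHealth on the main game mode.
; Overlapping fix_part actors are destroyed by PartNumber, with some revealing part meshes, but only parts 1 and 2 raise PartCount.
; Tick runs Checkfix, which clears the broken state at two counted parts and otherwise keeps all three pieces hidden while broken.
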(event `self.ReceiveTick`
  (params (DeltaSeconds :type "Float (single-precision)"))
  (`self.checkfix`))

(event `brok`
  (bind _output_get (set `self.broken` true))
  (if _output_get
    (set `self.is_oxy_fix` false)
    (bind _asmain (cast `/Game/Test_Farm/Blueprint/main` (`GameplayStatics.GetGameMode`)))
    (set `/Game/Test_Farm/Blueprint/main.bunker_health` (/ (`/Game/Test_Farm/Blueprint/main.bunker_health` _asmain) 2) _asmain)))

(event `self.Box.OnComponentBeginOverlap`
  (params (OverlappedComponent :type "PrimitiveComponent Object Reference") (OtherActor :type "Actor Object Reference") (OtherComp :type "PrimitiveComponent Object Reference") (OtherBodyIndex :type Integer) (bFromSweep :type Boolean) (SweepResult :type "HitResult Structure (by ref)"))
  (bind _asfix_part (cast `/Game/Test_Farm/Blueprint/fix_part` OtherActor))
  (switch `int` (`/Game/Test_Farm/Blueprint/fix_part.part_number` _asfix_part)
    (:`1`
      (`SceneComponent.SetHiddenInGame` (`self.path1`) false false)
      (`self.K2_DestroyActor` OtherActor :!label _label)
      (set `self.part_count` (+ (`self.part_count`) 1)))
    (:`2`
      (`SceneComponent.SetHiddenInGame` (`self.path2`) false false)
      (goto _label))
    (:`3`
      (`SceneComponent.SetHiddenInGame` (`self.part3`) false false)
      (`self.K2_DestroyActor` OtherActor))
    (:`4`
      (`self.K2_DestroyActor` OtherActor))))

(fn `checkfix`
  (if (`self.broken`)
    (if (>= (`self.part_count`) 2)
      (set `self.broken` false)
      (set `self.is_oxy_fix` true)
      (else
        (set `self.broken` true)
        (set `self.is_oxy_fix` false)
        (`SceneComponent.SetHiddenInGame` (`self.path1`) true false)
        (`SceneComponent.SetHiddenInGame` (`self.path2`) true false)
        (`SceneComponent.SetHiddenInGame` (`self.part3`) true false)))))

(fn `UserConstructionScript`)