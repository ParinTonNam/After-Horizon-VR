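; Test crop plot actor for a farm that starts growing a pumpkin when a Hoe touches it.
; A Hoe overlapping the Box swaps the soil material, then timed Delays step the Plant mesh through three pumpkin stages.
; Other overlapping actors only print a debug message.
; A separate SoilPlant function sets the Plant mesh by index from PlantList1, but the overlap chain does not call it.
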(event `self.ReceiveActorBeginOverlap`
  (params (OtherActor :type "Actor Object Reference")))

(event `self.Box.OnComponentBeginOverlap`
  (params (OverlappedComponent :type "PrimitiveComponent Object Reference") (OtherActor :type "Actor Object Reference") (OtherComp :type "PrimitiveComponent Object Reference") (OtherBodyIndex :type Integer) (bFromSweep :type Boolean) (SweepResult :type "HitResult Structure (by ref)"))
  (cast `/Game/Test_Farm/Blueprint/Hoe` OtherActor
    (:`then`
      (`KismetSystemLibrary.PrintString` "Hello hoe")
      (`PrimitiveComponent.SetMaterial` (`self.StaticMesh`) 1 "/Game/FarmCrops/MaterialInstances/MI_PlanterSoil_01.MI_PlanterSoil_01")
      (`KismetSystemLibrary.Delay` 10.0)
      (`StaticMeshComponent.SetStaticMesh` (`self.plant`) "/Game/FarmCrops/Meshes/Crops/SM_Pumpkin_01.SM_Pumpkin_01")
      (`KismetSystemLibrary.Delay` 10.0)
      (`StaticMeshComponent.SetStaticMesh` (`self.plant`) "/Game/FarmCrops/Meshes/Crops/SM_Pumpkin_02.SM_Pumpkin_02")
      (`KismetSystemLibrary.Delay` 10.0)
      (`StaticMeshComponent.SetStaticMesh` (`self.plant`) "/Game/FarmCrops/Meshes/Crops/SM_Pumpkin_03.SM_Pumpkin_03"))
    (:`CastFailed`
      (`KismetSystemLibrary.PrintString` "NO Hoe"))))

(fn `soil_plant`
  (params (NewParam :type Integer))
  (`StaticMeshComponent.SetStaticMesh` (`self.plant`) (`|GetArrayItem` (`self.plant_list_1`) NewParam)))

(fn `UserConstructionScript`)